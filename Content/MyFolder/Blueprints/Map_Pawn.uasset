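; Pawn for a map screen that hops between points of interest and opens the level attached to the current one.
; It starts at CurrentPOI, and directional move inputs snap it to that POI's north, south, east or west neighbour, when valid, then make that neighbour current.
; The Next Level input opens the level named on the current POI.
; Disconnected leftover nodes from an index-based cycling approach never run.
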(event `self.ReceiveBeginPlay`
  (`self.K2_SetActorLocation` (`self.K2_GetActorLocation` (`self.CurrentPOI`))))

(event `InputAction|Move East`
  (params (Key :type "Key Structure"))
  (bind _poi_e (`/Game/MyFolder/Blueprints/POI_BP.POI_E` (`self.CurrentPOI`)))
  ;[1 1 1] Cycle Through
  (:`Pressed`
    (if (`KismetSystemLibrary.IsValid` _poi_e)
      (`self.K2_SetActorLocation` (`self.K2_GetActorLocation` _poi_e))
      (set `self.CurrentPOI` (`/Game/MyFolder/Blueprints/POI_BP.POI_E` (`self.CurrentPOI`))))))

(event `InputAction|Move West`
  (params (Key :type "Key Structure"))
  (bind _poi_w (`/Game/MyFolder/Blueprints/POI_BP.POI_W` (`self.CurrentPOI`)))
  ;[1 1 1] Cycle Through
  (:`Pressed`
    (if (`KismetSystemLibrary.IsValid` _poi_w)
      (`self.K2_SetActorLocation` (`self.K2_GetActorLocation` _poi_w))
      (set `self.CurrentPOI` (`/Game/MyFolder/Blueprints/POI_BP.POI_W` (`self.CurrentPOI`))))))

(event `InputAction|Move North`
  (params (Key :type "Key Structure"))
  (bind _poi_n (`/Game/MyFolder/Blueprints/POI_BP.POI_N` (`self.CurrentPOI`)))
  ;[1 1 1] Cycle Through
  (:`Pressed`
    (if (`KismetSystemLibrary.IsValid` _poi_n)
      (`self.K2_SetActorLocation` (`self.K2_GetActorLocation` _poi_n))
      (set `self.CurrentPOI` (`/Game/MyFolder/Blueprints/POI_BP.POI_N` (`self.CurrentPOI`))))))

(event `InputAction|Move South`
  (params (Key :type "Key Structure"))
  (bind _poi_s (`/Game/MyFolder/Blueprints/POI_BP.POI_S` (`self.CurrentPOI`)))
  ;[1 1 1] Cycle Through
  (:`Pressed`
    (if (`KismetSystemLibrary.IsValid` _poi_s)
      (`self.K2_SetActorLocation` (`self.K2_GetActorLocation` _poi_s))
      (set `self.CurrentPOI` (`/Game/MyFolder/Blueprints/POI_BP.POI_S` (`self.CurrentPOI`))))))

(event `InputAction|Next Level`
  (params (Key :type "Key Structure"))
  (:`Pressed`
    (`GameplayStatics.OpenLevel` (`/Game/MyFolder/Blueprints/POI_BP.LevelToOpen` (`self.CurrentPOI`)))))

(fn `UserConstructionScript`)