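; Player character for a 2D side-scroller with running, jumping, shooting, climbing and damage, plus a HUD widget.
; A state enum selects the sprite flipbook, refreshed on Tick, which also turns the controller to face movement.
; Damage disables input and either kills or applies knockback and a blink timer; landing after a hit restores control.
; Shoot and ClimbUp share one branch that climbs or spawns a shot, depending on Climb.
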(event `self.ReceiveBeginPlay`
  ;[1 0.02482 0.8704] Initialize
  (`|ExecutionSequence`
    (:`then_0`
      (`ActorComponent.SetIsReplicated` (`self.Sprite`) true))
    (:`then_1`
      (bind _returnvalue (`|CreateWidget` "/Game/MyFolder/Blueprints/Wideget_HUD.Wideget_HUD_C" (`GameplayStatics.GetPlayerController` 0)))
      (bind _output_get (set `self.W_HealthBar` _returnvalue))
      (`UserWidget.AddToViewport` _output_get 0))))

(event `CE_Blink`
  ;[1 0.1235 0.1732] Event Blink
  (`SceneComponent.SetHiddenInGame` (`self.Sprite`) true false)
  (`KismetSystemLibrary.Delay` 1.0)
  (`SceneComponent.SetHiddenInGame` (`self.Sprite`) false false))

(event `CE_Damage_System`
  (params (DamageIn :type "Float (double-precision)"))
  ;[1 0.1291 0.2108] Deal Damage
  (set `self.IsHit` true :!label _label)
  (`self.DisableInput` (`GameplayStatics.GetPlayerController` 0))
  (bind _output_get (set `self.HealthCurrent` (- (`self.HealthCurrent`) DamageIn)))
  (if (<= _output_get 0.0)
    (set `self.E_CharState` "NewEnumerator5")
    (`self.DisableInput` (`GameplayStatics.GetPlayerController` 0))
    (else
      (set `self.E_CharState` "NewEnumerator4")
      (`CharacterMovementComponent.AddForce` (`self.CharacterMovement`) (`KismetMathLibrary.MakeVector` (* (`self.Facing`) (`self.KnockBack`)) 0.0 2000000.0))
      (`KismetSystemLibrary.K2_SetTimer` null "Blink" 2.0 true))))

(event `Key|Backslash`
  (params (Key :type "Key Structure"))
  ;[1 0.1291 0.2108] Deal Damage
  (:`Pressed`
    (goto _label)))

(event `self.OnLanded`
  (params (Hit :type "HitResult Structure (by ref)"))
  ;[1 0.1306 0.1963] Event On_Landed
  (if (`self.IsHit`)
    (set `self.E_CharState` "NewEnumerator6")
    (`self.CE_UpdateAnimation`)
    (`KismetSystemLibrary.Delay` 0.5)
    (set `self.IsHit` false)
    (set `self.E_CharState` "NewEnumerator0")
    (`self.CE_UpdateAnimation`)
    (`self.EnableInput` (`GameplayStatics.GetPlayerController` 0))
    (else
      (set `self.E_CharState` "NewEnumerator0")
      (`self.CE_UpdateAnimation`))))

(event `InputAction|Jump`
  (params (Key :type "Key Structure"))
  ;[1 0.98 0.5857] Handle Jump
  (:`Pressed`
    (`self.Jump` :!label _label_2)
    (set `self.E_CharState` "NewEnumerator2"))
  (:`Released`
    (`self.StopJumping` :!label _label_3)))

(event `CE_UpdateAnimation`
  ;[1 0.9629 0.3573] Handle Animation
  (switch `/Game/MyFolder/Blueprints/E_Char_States` (`self.E_CharState`)
    (:`NewEnumerator0`
      (`PaperFlipbookComponent.SetFlipbook` (`self.Sprite`) (select `bool` (> (`KismetMathLibrary.VSize` (`self.GetVelocity`)) 0.0) :`false` "/Game/MyFolder/Sprites/Character/A_Stance.A_Stance" :`true` "/Game/MyFolder/Sprites/Character/A_Run.A_Run" :!type "PaperFlipbook Object Reference")))
    (:`NewEnumerator2`
      (`PaperFlipbookComponent.SetFlipbook` (`self.Sprite`) "/Game/MyFolder/Sprites/Character/A_Jump.A_Jump"))
    (:`NewEnumerator4`
      (`PaperFlipbookComponent.SetFlipbook` (`self.Sprite`) "/Game/MyFolder/Sprites/Character/A_Hit.A_Hit"))
    (:`NewEnumerator5`
      (`PaperFlipbookComponent.SetFlipbook` (`self.Sprite`) "/Game/MyFolder/Sprites/Character/A_Dead.A_Dead"))
    (:`NewEnumerator6`
      (`PaperFlipbookComponent.SetFlipbook` (`self.Sprite`) "/Game/MyFolder/Sprites/Character/A_Sitting.A_Sitting"))
    (:`NewEnumerator7`
      (`PaperFlipbookComponent.SetFlipbook` (`self.Sprite`) "/Game/MyFolder/Sprites/Character/A_Shoot.A_Shoot"))))

(event `InputTouch`
  (params (Location :type "Vector Structure") (FingerIndex :type "ETouchIndex Enum"))
  ;[1 0.98 0.5857] Handle Jump
  (:`Pressed`
    (goto _label_2))
  (:`Released`
    (goto _label_3)))

(event `InputAxis|MoveRight`
  (params (AxisValue :type "Float (single-precision)"))
  ;[0.9015 1 0.5118] Handle movement
  (if (`self.Move`)
    (if (> AxisValue 0.0)
      (set `self.bisMovingRight` true)
      (elif (< AxisValue 0.0)
        (set `self.bisMovingRight` false)))
    (`self.AddMovementInput` (1.0 0.0 0.0) AxisValue)))

(event `self.ReceiveTick`
  (params (DeltaSeconds :type "Float (single-precision)"))
  (bind _returnvalue (`self.GetController`))
  (bind _returnvalue_2 (`self.GetController`))
  ;[0.9425 0.01054 1] Tick - Updates animation
  (`self.CE_UpdateAnimation`)
  ;;[1 0.9832 0.5301] Handle Orientation
  (`/Engine/EditorBlueprintResources/StandardMacros.CompareFloat` (.x (`MovementComponent.Velocity` (`self.GetMovementComponent`)))
    (:`>`
      (`/Engine/EditorBlueprintResources/StandardMacros.IsValid` _returnvalue_2 :!label _label_4
        (:`Is Valid`
          (`Controller.SetControlRotation` _returnvalue_2 (`KismetMathLibrary.MakeRotator` 0.0))
          (set `self.Facing` 1))))
    (:`==`
      (if (`self.bisMovingRight`)
        (goto _label_4)
        (else
          (`/Engine/EditorBlueprintResources/StandardMacros.IsValid` _returnvalue :!label _label_5
            (:`Is Valid`
              (`Controller.SetControlRotation` _returnvalue (`KismetMathLibrary.MakeRotator` 0.0 0.0 180.0))
              (set `self.Facing` -1))))))
    (:`<`
      (goto _label_5))))

(event `InputAction|Shoot`
  (params (Key :type "Key Structure"))
  (:`Pressed`
    (if (`self.Climb`) :!label _label_6
      (bind _returnvalue (* (stale `InputAxis|ClimbUp` AxisValue) (`self.ClimbSpeed`)))
      (`KismetSystemLibrary.PrintString` (`KismetStringLibrary.Conv_DoubleToString` _returnvalue))
      (`self.K2_AddActorLocalOffset` (`KismetMathLibrary.MakeVector` 0.0 0.0 _returnvalue))
      (else
        (set `self.Move` false)
        (`|SpawnActorFromClass` "/Game/MyFolder/Blueprints/BP_Shot.BP_Shot_C" (`SceneComponent.K2_GetComponentToWorld` (`self.Arrow1`)) "AlwaysSpawn" "OverrideRootScale" null null)
        (set `self.E_CharState` "NewEnumerator7")
        (`MovementComponent.StopMovementImmediately` (`self.CharacterMovement`))
        (`self.CE_UpdateAnimation` :!label _label_7))))
  (:`Released`
    (`KismetSystemLibrary.RetriggerableDelay` 0.2)
    (set `self.E_CharState` "NewEnumerator0")
    (set `self.Move` true)
    (goto _label_7)))

(event `InputAxis|ClimbUp`
  (params (AxisValue :type "Float (single-precision)"))
  (if (>= AxisValue 0.1)
    (goto _label_6)))

(fn `UserConstructionScript`)